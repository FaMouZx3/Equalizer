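; Scaler is an audio spectrum visualizer that plays a sound and scales placed Visualizer actors as equalizer bars.
; On BeginPlay it collects the Visualizer actors into EqBars, insertion-sorted by X position, and starts the audio.
; Each Tick it samples the sound's frequency spectrum, using game time as the playback offset, and maps each band to the clamped Z scale of its bar.
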(event Custom|BreakLoop
  (bind _eqbars (Variables|Default|GetEqBars))
  (Utilities|Array|ForEachLoopwithBreak _eqbars) ; enters at Break
)

(event EventBeginPlay
  (bind _eqbars (Variables|Default|GetEqBars))
  (bind _outactors (Actor|GetAllActorsOfClass "/Game/Blueprints/Visualizer.Visualizer_C"))
  (for _array_element _outactors
    (bind (_array_element_2 _array_index) (Utilities|Array|ForEachLoopwithBreak _eqbars)
      (:LoopBody
        (if (not (< (.X (Math|Vector|BreakVector (Transformation|GetActorLocation _array_element_2))) (.X (Math|Vector|BreakVector (Transformation|GetActorLocation _array_element)))))
          (CallFunction|BreakLoop)))
      (:Completed
        (Utilities|Array|Insert _eqbars _array_element _array_index))))
  (Audio|Components|Audio|SetSound (Variables|Default|GetAudio) (Variables|Default|GetSound))
  (Audio|Components|Audio|Play (Variables|Default|GetAudio) 0.0))

(event EventTick
  (params (DeltaSeconds :type Float%20%28single-precision%29))
  (bind _outspectrum (Class|SoundVisualizationStatics|CalculateFrequencySpectrum (Variables|Default|GetSound) 0 (Utilities|Time|GetGameTimeinSeconds) 0.19 28))
  (Variables|Default|SetFrequences _outspectrum)
  (for (_array_element _array_index) (Variables|Default|GetEqBars)
    (Transformation|SetActorScale3D _array_element (Math|Vector|MakeVector 0.8 0.8 (Math|Float|Clamp(Float) (/ (Utilities|Array|Get(acopy) (Variables|Default|GetFrequences) _array_index) 8.0) 0.1 1e+01)))))

(fn ConstructionScript)